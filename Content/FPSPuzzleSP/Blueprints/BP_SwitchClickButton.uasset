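; BP_SwitchClickButton is a puzzle switch that the player toggles by pressing interact, sending on/off messages to linked actors.
; Each Tick, when nearby with interact active, it traces for a switch and flips that switch's StartedState if Availible is set.
; Event swaps the material, calls TurnMessage and plays a sound for each OutputTo entry, then restores Availible after a delay.
; BeginPlay runs the same logic to broadcast the initial state.
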(event Custom|Event
  (bind _staticmesh (Variables|Default|GetStaticMesh))
  (bind _output_to_ (Variables|Default|GetOutput%20to:))
  (if (Variables|Default|GetStartedState)
    (Rendering|Material|SetMaterial _staticmesh 1 "/Game/FPSPuzzleSP/Materials/Instance/MI_SwitchOn.MI_SwitchOn")
    (for _array_element _output_to_
      (Class|BISignal|Turn(Message) _array_element "NewEnumerator0")
      (CallFunction|PlaySoundbyDataTable "BP_SwitchClickButton" (Transformation|GetActorLocation) 0.2))
    (else
      (Rendering|Material|SetMaterial _staticmesh 1 "/Game/FPSPuzzleSP/Materials/Instance/MI_SwitchOff.MI_SwitchOff")
      (for _array_element_2 _output_to_
        (Class|BISignal|Turn(Message) _array_element_2 "NewEnumerator1")
        (CallFunction|PlaySoundbyDataTable "BP_SwitchClickButton" (Transformation|GetActorLocation) 0.2))))
  (Utilities|FlowControl|Delay 1.0)
  (Variables|Default|SetAvailible true))

(event EventBeginPlay
  (bind _staticmesh (Variables|Default|GetStaticMesh))
  (bind _output_to_ (Variables|Default|GetOutput%20to:))
  (if (Variables|Default|GetStartedState)
    (Rendering|Material|SetMaterial _staticmesh 1 "/Game/FPSPuzzleSP/Materials/Instance/MI_SwitchOn.MI_SwitchOn")
    (for _array_element _output_to_
      (Class|BISignal|Turn(Message) _array_element "NewEnumerator0")
      (CallFunction|PlaySoundbyDataTable "BP_SwitchClickButton" (Transformation|GetActorLocation) 0.2))
    (else
      (Rendering|Material|SetMaterial _staticmesh 1 "/Game/FPSPuzzleSP/Materials/Instance/MI_SwitchOff.MI_SwitchOff")
      (for _array_element_2 _output_to_
        (Class|BISignal|Turn(Message) _array_element_2 "NewEnumerator1")
        (CallFunction|PlaySoundbyDataTable "BP_SwitchClickButton" (Transformation|GetActorLocation) 0.2))))
  (Utilities|FlowControl|Delay 1.0)
  (Variables|Default|SetAvailible true))

(event EventTick
  (params (DeltaSeconds :type Float%20%28single-precision%29))
  (bind _is_near (CallFunction|ActorIsNear self 1e+03))
  (if _is_near
    (if (Input|EnhancedActionValues|GetIA_Interact)
      (bind _hitactor (CallFunction|TracefromActor (Variables|Default|GetDitantionForPress) "TraceTypeQuery1" false (Utilities|Array|MakeArray (Game|Player|GetPlayerPawn 0)) false)) ; FL_PuzzleLib
      (bind _asbp_switch_click_button (Utilities|Casting|CastToBP_SwitchClickButton _hitactor))
      (if (Variables|Default|GetAvailible)
        (Variables|Default|SetAvailible false)
        (Variables|BP_SwitchClickButton_C|SetStartedState _asbp_switch_click_button (not (Variables|BP_SwitchClickButton_C|GetStartedState _asbp_switch_click_button)))
        (CallFunction|Event _asbp_switch_click_button)))))

(fn ConstructionScript
  (bind _returnvalue (Rendering|Material|CreateDynamicMaterialInstance "/Game/FPSPuzzleSP/Materials/Instance/MI_SwitchOn.MI_SwitchOn" "None" "None" :!class /Script/Engine.KismetMaterialLibrary))
  (bind _output_get (Variables|Default|SetMaterial _returnvalue))
  (Rendering|Material|SetMaterial (Variables|Default|GetStaticMesh) 1 _output_get))